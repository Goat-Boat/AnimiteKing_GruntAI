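; Elite melee grunt enemy Blueprint that supplies a randomized Melee attack.
; The Melee event switches on a random integer to play one of the attack montages at reduced speed, then after a short delay calls Attack on one of two hitboxes.
; The random range yields only 0 to 2, so the fourth montage, Attack D, is never selected.
; The construction script only calls its parent.
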(event `/Game/EnemyAI/BasicEnemy.Melee`
  (bind _hitbox2 (`self.Hitbox2`))
  (bind _hitbox1 (`self.Hitbox1`))
  (switch `int` (`KismetMathLibrary.RandomInteger` 3)
    (:`Default`
      (`self.PlayAnimMontage` "/Game/EnemyAI/MeleeEnemy/Animations/Attack_D_Montage.Attack_D_Montage" 0.75 :!label _label)
      (`KismetSystemLibrary.Delay` 0.35)
      (`/Game/EnemyAI/MeleeEnemy/Blueprints/MeleeHitbox.Attack` _hitbox2))
    (:`0`
      (`self.PlayAnimMontage` "/Game/EnemyAI/MeleeEnemy/Animations/Attack_A_Montage.Attack_A_Montage" 0.75)
      (`KismetSystemLibrary.Delay` 0.35)
      (`/Game/EnemyAI/MeleeEnemy/Blueprints/MeleeHitbox.Attack` _hitbox1))
    (:`1`
      (`self.PlayAnimMontage` "/Game/EnemyAI/MeleeEnemy/Animations/Attack_B_Montage.Attack_B_Montage" 0.75)
      (`KismetSystemLibrary.Delay` 0.35)
      (`/Game/EnemyAI/MeleeEnemy/Blueprints/MeleeHitbox.Attack` _hitbox2))
    (:`2`
      (`self.PlayAnimMontage` "/Game/EnemyAI/MeleeEnemy/Animations/Attack_C_Montage.Attack_C_Montage" 0.75)
      (`KismetSystemLibrary.Delay` 0.35)
      (`/Game/EnemyAI/MeleeEnemy/Blueprints/MeleeHitbox.Attack` _hitbox1))
    (:`3`
      (goto _label))))

(fn `UserConstructionScript`
  (`parent.UserConstructionScript`))