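; Melee grunt enemy that attacks with two socket-attached hitboxes and handles its own death.
; BeginPlay spawns both hitboxes, snaps them to mesh sockets and gives them the base damage.
; Melee plays a random attack montage, then triggers its paired hitbox after a short delay; RandomInteger(3) leaves Attack_D unreachable.
; Death clears aggro, plays the death animation and destroys the actor after a delay.
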(event `self.ReceiveBeginPlay`
  (bind _returnvalue (`SceneComponent.K2_GetComponentToWorld` (`self.Mesh`)))
  (bind _returnvalue_2 (`|SpawnActorFromClass` "/Game/EnemyAI/MeleeEnemy/Blueprints/MeleeHitbox.MeleeHitbox_C" _returnvalue "AlwaysSpawn" "OverrideRootScale" null null))
  (bind _output_get (set `self.Hitbox1` _returnvalue_2))
  (`self.K2_AttachToComponent` _output_get (`self.Mesh`) "MeleeSocket1" "SnapToTarget" "SnapToTarget" "SnapToTarget" true)
  (bind _returnvalue_3 (`|SpawnActorFromClass` "/Game/EnemyAI/MeleeEnemy/Blueprints/MeleeHitbox.MeleeHitbox_C" _returnvalue "AlwaysSpawn" "OverrideRootScale" null null))
  (bind _output_get_2 (set `self.Hitbox2` _returnvalue_3))
  (`self.K2_AttachToComponent` _output_get_2 (`self.Mesh`) "MeleeSocket2" "SnapToTarget" "SnapToTarget" "SnapToTarget" true)
  (`/Game/EnemyAI/MeleeEnemy/Blueprints/MeleeHitbox.SetDamage` (`self.Hitbox2`) (`self.BaseDamage`))
  (`/Game/EnemyAI/MeleeEnemy/Blueprints/MeleeHitbox.SetDamage` (`self.Hitbox1`) (`self.BaseDamage`)))

(event `self.Death`
  (set `self.HasAggro` false)
  (`SkeletalMeshComponent.PlayAnimation` (`self.Mesh`) "/Game/EnemyAI/MeleeEnemy/Animations/Death_A.Death_A" false)
  (`KismetSystemLibrary.Delay` 3.0)
  (`self.K2_DestroyActor`))

(event `self.Melee`
  (bind _hitbox2 (`self.Hitbox2`))
  (bind _hitbox1 (`self.Hitbox1`))
  (switch `int` (`KismetMathLibrary.RandomInteger` 3)
    (:`Default`
      (`self.PlayAnimMontage` "/Game/EnemyAI/MeleeEnemy/Animations/Attack_D_Montage.Attack_D_Montage" :!label _label)
      (`KismetSystemLibrary.Delay` 0.3)
      (`/Game/EnemyAI/MeleeEnemy/Blueprints/MeleeHitbox.Attack` _hitbox2))
    (:`0`
      (`self.PlayAnimMontage` "/Game/EnemyAI/MeleeEnemy/Animations/Attack_A_Montage.Attack_A_Montage")
      (`KismetSystemLibrary.Delay` 0.3)
      (`/Game/EnemyAI/MeleeEnemy/Blueprints/MeleeHitbox.Attack` _hitbox1))
    (:`1`
      (`self.PlayAnimMontage` "/Game/EnemyAI/MeleeEnemy/Animations/Attack_B_Montage.Attack_B_Montage")
      (`KismetSystemLibrary.Delay` 0.3)
      (`/Game/EnemyAI/MeleeEnemy/Blueprints/MeleeHitbox.Attack` _hitbox2))
    (:`2`
      (`self.PlayAnimMontage` "/Game/EnemyAI/MeleeEnemy/Animations/Attack_C_Montage.Attack_C_Montage")
      (`KismetSystemLibrary.Delay` 0.3)
      (`/Game/EnemyAI/MeleeEnemy/Blueprints/MeleeHitbox.Attack` _hitbox1))
    (:`3`
      (goto _label))))

(fn `UserConstructionScript`
  (`parent.UserConstructionScript`))