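; MeleeHitbox is the damage volume for a melee enemy's attack, with its collision disabled on construction.
; Attack enables query-only collision on the Hitbox for a one-second window, then disables it.
; An overlapping Player receives the Damage value, supplied through SetDamage, via ChangeHealth.
; The hitbox switches off right after that hit, limiting each swing to one damage application.
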(event `Attack`
  (`PrimitiveComponent.SetCollisionEnabled` (`self.Hitbox`) "QueryOnly")
  (`KismetSystemLibrary.Delay` 1.0)
  (`PrimitiveComponent.SetCollisionEnabled` (`self.Hitbox`) "NoCollision"))

(event `SetDamage`
  (params (Damage :type "Float (double-precision)"))
  (set `self.Damage` Damage))

(event `self.Hitbox.OnComponentBeginOverlap`
  (params (OverlappedComponent :type "PrimitiveComponent Object Reference") (OtherActor :type "Actor Object Reference") (OtherComp :type "PrimitiveComponent Object Reference") (OtherBodyIndex :type Integer) (bFromSweep :type Boolean) (SweepResult :type "HitResult Structure (by ref)"))
  (bind _asplayer (cast `/Game/Blueprints/Player` OtherActor))
  (`/Game/Blueprints/Player.ChangeHealth` _asplayer (`self.Damage`))
  (`PrimitiveComponent.SetCollisionEnabled` (`self.Hitbox`) "NoCollision"))

(fn `UserConstructionScript`
  (`PrimitiveComponent.SetCollisionEnabled` (`self.Hitbox`) "NoCollision"))