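; Ranged grunt enemy that turns to face the player every tick while it has aggro, with ranged, melee and death events.
; Fire plays a bow montage and spawns an EnemyProjectile at Arrow1.
; Melee briefly enables a collision that passes BaseDamage to the player's health, launches them, then switches off.
; Death clears aggro, plays an animation and destroys the actor after a delay.
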(event `self.ReceiveTick`
  (params (DeltaSeconds :type "Float (single-precision)"))
  (if (`self.HasAggro`)
    (`self.K2_SetActorRotation` (`KismetMathLibrary.FindLookAtRotation` (`self.K2_GetActorLocation`) (`self.K2_GetActorLocation` (`GameplayStatics.GetPlayerCharacter` 0))))))

(event `self.Death`
  (set `self.HasAggro` false)
  (`SkeletalMeshComponent.PlayAnimation` (`self.Mesh`) "/Game/EnemyAI/RangedEnemy/Animations/Standing_Death1.Standing_Death1" false)
  (`KismetSystemLibrary.Delay` 3.0)
  (`self.K2_DestroyActor`))

(event `self.Fire`
  (`self.PlayAnimMontage` "/Game/EnemyAI/RangedEnemy/Animations/ShootArrow_Montage.ShootArrow_Montage")
  (`|SpawnActorFromClass` "/Game/EnemyAI/RangedEnemy/Blueprints/EnemyProjectile.EnemyProjectile_C" (`SceneComponent.K2_GetComponentToWorld` (`self.Arrow1`)) "AlwaysSpawn" "OverrideRootScale" null null))

(event `self.Melee`
  (`self.PlayAnimMontage` "/Game/EnemyAI/RangedEnemy/Animations/Standing_Melee_Punch_Montage.Standing_Melee_Punch_Montage")
  (`PrimitiveComponent.SetCollisionEnabled` (`self.MeleeCollision`) "QueryOnly")
  (`KismetSystemLibrary.Delay` 1.0)
  (`PrimitiveComponent.SetCollisionEnabled` (`self.MeleeCollision`) "NoCollision"))

(event `self.ReceiveBeginPlay`
  (`parent.ReceiveBeginPlay`))

(event `self.MeleeCollision.OnComponentBeginOverlap`
  (params (OverlappedComponent :type "PrimitiveComponent Object Reference") (OtherActor :type "Actor Object Reference") (OtherComp :type "PrimitiveComponent Object Reference") (OtherBodyIndex :type Integer) (bFromSweep :type Boolean) (SweepResult :type "HitResult Structure (by ref)"))
  (bind _asplayer (cast `/Game/Blueprints/Player` OtherActor))
  (`/Game/Blueprints/Player.ChangeHealth` _asplayer (`self.BaseDamage`))
  (`self.LaunchCharacter` _asplayer (+ (* (`self.GetActorForwardVector`) 500) (`KismetMathLibrary.MakeVector` 0.0 100.0 100.0)) false false)
  (`PrimitiveComponent.SetCollisionEnabled` (`self.MeleeCollision`) "NoCollision"))

(fn `UserConstructionScript`
  (`parent.UserConstructionScript`)
  (`PrimitiveComponent.SetCollisionEnabled` (`self.MeleeCollision`) "NoCollision"))