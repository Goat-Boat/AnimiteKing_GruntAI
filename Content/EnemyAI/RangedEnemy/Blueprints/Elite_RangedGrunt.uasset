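; Elite ranged grunt enemy character that provides fire, melee and death actions as events.
; Fire plays the shoot montage, then after a short delay spawns an elite projectile at the arrow component's transform.
; Melee plays a punch montage and enables query collision on the melee hitbox, with no disable in this graph.
; Death clears aggro, plays the death animation and destroys the actor after a delay.
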(event `self.Death`
  (set `self.HasAggro` false)
  (`SkeletalMeshComponent.PlayAnimation` (`self.Mesh`) "/Game/EnemyAI/RangedEnemy/Animations/Elite/Elite_Ranged_Death.Elite_Ranged_Death" false)
  (`KismetSystemLibrary.Delay` 3.0)
  (`self.K2_DestroyActor`))

(event `self.Fire`
  (`self.PlayAnimMontage` "/Game/EnemyAI/RangedEnemy/Animations/Elite/Elite_Ranged_Shoot_Montage.Elite_Ranged_Shoot_Montage")
  (`KismetSystemLibrary.Delay` 0.25)
  (`|SpawnActorFromClass` "/Game/EnemyAI/RangedEnemy/Blueprints/Elite_EnemyProjectile.Elite_EnemyProjectile_C" (`SceneComponent.K2_GetComponentToWorld` (`self.Arrow1`)) "AlwaysSpawn" "OverrideRootScale" null null))

(event `self.Melee`
  (`self.PlayAnimMontage` "/Game/EnemyAI/RangedEnemy/Animations/Elite/Elite_Ranged_Punch_Montage.Elite_Ranged_Punch_Montage")
  (`PrimitiveComponent.SetCollisionEnabled` (`self.MeleeCollision`) "QueryOnly"))

(fn `UserConstructionScript`
  (`parent.UserConstructionScript`))