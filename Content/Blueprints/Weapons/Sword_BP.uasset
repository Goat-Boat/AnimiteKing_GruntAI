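; Sword weapon Blueprint that damages BasicEnemy actors it overlaps during an attack.
; Collision starts disabled in the construction script, and Attack turns it on as query-only after a short windup, then off again after a fixed window.
; The overlap event applies Damage to a BasicEnemy and disables collision at once, so each swing normally hits only one enemy.
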(event `Attack`
  (`KismetSystemLibrary.Delay` 0.2)
  (`PrimitiveComponent.SetCollisionEnabled` (`self.Collision`) "QueryOnly")
  (`KismetSystemLibrary.Delay` 1.0)
  (`PrimitiveComponent.SetCollisionEnabled` (`self.Collision`) "NoCollision"))

(event `self.Collision.OnComponentBeginOverlap`
  (params (OverlappedComponent :type "PrimitiveComponent Object Reference") (OtherActor :type "Actor Object Reference") (OtherComp :type "PrimitiveComponent Object Reference") (OtherBodyIndex :type Integer) (bFromSweep :type Boolean) (SweepResult :type "HitResult Structure (by ref)"))
  (bind _asbasic_enemy (cast `/Game/EnemyAI/BasicEnemy` OtherActor))
  (`/Game/EnemyAI/BasicEnemy.TakeDamage` _asbasic_enemy (`self.Damage`))
  (`PrimitiveComponent.SetCollisionEnabled` (`self.Collision`) "NoCollision"))

(fn `UserConstructionScript`
  (`parent.UserConstructionScript`)
  (`PrimitiveComponent.SetCollisionEnabled` (`self.Collision`) "NoCollision"))