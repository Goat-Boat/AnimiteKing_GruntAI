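; Engineer shield actor that absorbs enemy projectiles while reserving some of the player's mana.
; On spawn it copies the player's max health, raises ManaReduction, clears ShieldDown and attaches an emitter, removed by a delay polling loop upon death.
; Overlapping mage and bullet projectiles deduct their damage and are destroyed.
; Tick detects depleted health, hides the mesh, then after a cooldown releases the mana, sets ShieldDown and destroys the actor.
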(event `self.ReceiveBeginPlay`
  ;[1 1 1] On creation
  (set `self.IsAlive` true)
  (bind _asplayer (cast `/Game/Blueprints/Player` (`GameplayStatics.GetPlayerCharacter` 0)))
  (if (not (`self.HealthSet`))
    (set `/Game/Blueprints/Player.ManaReduction` (+ (`self.ManaHold`) (`/Game/Blueprints/Player.ManaReduction` _asplayer)) _asplayer)
    (set `self.Health` (`/Game/Blueprints/Player.MaxHealth` _asplayer))
    (set `self.HealthSet` true)
    (set `/Game/Blueprints/Player.ShieldDown` false _asplayer)
    (bind _returnvalue (`GameplayStatics.SpawnEmitterAttached` null (`self.StaticMesh`) "None" (0.0 0.0 50.0)))
    (bind _output_get (set `self.Emitter Reference` _returnvalue))
    (if (`self.IsAlive`) :!label _label
      (`KismetSystemLibrary.Delay` 0.1)
      (goto _label)
      (else
        (`ActorComponent.K2_DestroyComponent` _output_get)))))

(event `self.ReceiveActorBeginOverlap`
  (params (OtherActor :type "Actor Object Reference"))
  ;[1 1 1] Shield Take Damage
  (if (`self.IsAlive`)
    (bind _asuhouse_enemy_projectile_mage (cast `/Game/Blueprints/UhouseEnemyProjectileMage` OtherActor)
      (:`then`
        (set `self.Health` (- (`self.Health`) (`/Game/Blueprints/UhouseEnemyProjectileMage.ProjDamage` _asuhouse_enemy_projectile_mage)))
        (`self.K2_DestroyActor` _asuhouse_enemy_projectile_mage))
      (:`CastFailed`
        (bind _asuhouse_enemy_projectile_bullet (cast `/Game/Blueprints/UhouseEnemyProjectileBullet` OtherActor))
        (set `self.Health` (- (`self.Health`) (`/Game/Blueprints/UhouseEnemyProjectileBullet.ProjDamage` _asuhouse_enemy_projectile_bullet)))
        (`self.K2_DestroyActor` _asuhouse_enemy_projectile_bullet)))))

(event `self.ReceiveTick`
  (params (DeltaSeconds :type "Float (single-precision)"))
  ;[1 1 1] Destroy Actor
  (if (<= (`self.Health`) 0.0)
    (set `self.IsAlive` false)
    (set `self.HealthSet` false)
    (`SceneComponent.SetVisibility` (`self.StaticMesh`) false false)
    (`KismetSystemLibrary.Delay` (`self.Cooldown`))
    (bind _asplayer (cast `/Game/Blueprints/Player` (`GameplayStatics.GetPlayerCharacter` 0)))
    (set `/Game/Blueprints/Player.ManaReduction` (- (`/Game/Blueprints/Player.ManaReduction` _asplayer) (`self.ManaHold`)) _asplayer)
    (set `/Game/Blueprints/Player.ShieldDown` true _asplayer)
    (`self.K2_DestroyActor`)))

(fn `UserConstructionScript`)