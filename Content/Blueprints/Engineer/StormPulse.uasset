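; StormPulse is an Engineer pulse actor that stuns overlapping enemies and gates the player's pulse through a PulseDown flag.
; BeginPlay clears that flag and attaches an emitter to the Sphere, then removes the emitter after a short fixed lifetime.
; Tick watches for the pulse's end, hides the Sphere, waits out Cooldown, then sets PulseDown and destroys the actor.
; The actor therefore outlives its visuals to serve as the cooldown timer.
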(event `self.ReceiveBeginPlay`
  ;[1 1 1] On Pulse Create
  (bind _asplayer (cast `/Game/Blueprints/Player` (`GameplayStatics.GetPlayerCharacter` 0)))
  (set `/Game/Blueprints/Player.PulseDown` false _asplayer)
  (set `self.Pulse_Exists` true)
  (bind _returnvalue (`GameplayStatics.SpawnEmitterAttached` null (`self.Sphere`) "None" (0.0 0.0 0.0) (struct) (0.75 0.75 0.75)))
  (bind _output_get (set `self.Emitter Ref` _returnvalue))
  (if (`self.Pulse_Exists`) :!label _label
    (`KismetSystemLibrary.Delay` 1.5)
    (set `self.Pulse_Exists` false)
    (goto _label)
    (else
      (`ActorComponent.K2_DestroyComponent` _output_get))))

(event `self.ReceiveActorBeginOverlap`
  (params (OtherActor :type "Actor Object Reference"))
  ;[1 1 1] On Enemy Overlap
  (bind _asuhouse_third_person_enemy (cast `/Game/Blueprints/UhouseThirdPersonEnemy` OtherActor))
  (if (not (`/Game/Blueprints/UhouseThirdPersonEnemy.Stunned` _asuhouse_third_person_enemy))
    (set `/Game/Blueprints/UhouseThirdPersonEnemy.Stunned` true _asuhouse_third_person_enemy)))

(event `self.ReceiveTick`
  (params (DeltaSeconds :type "Float (single-precision)"))
  ;[1 1 1] On Pulse Done
  (if (not (`self.Pulse_Exists`))
    (`SceneComponent.SetVisibility` (`self.Sphere`) false false)
    (`KismetSystemLibrary.Delay` (`self.Cooldown`))
    (bind _asplayer (cast `/Game/Blueprints/Player` (`GameplayStatics.GetPlayerCharacter` 0)))
    (set `/Game/Blueprints/Player.PulseDown` true _asplayer)
    (`self.K2_DestroyActor`)))

(fn `UserConstructionScript`)