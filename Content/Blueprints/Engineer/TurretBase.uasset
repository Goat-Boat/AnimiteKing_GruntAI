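; Engineer turret base actor that spawns a Turret and removes itself once that turret's health runs out.
; On BeginPlay it spawns the Turret at its own location with zero rotation and unit scale.
; Each Tick it takes the first overlapping Turret, rather than a stored reference to the spawned one, and destroys itself when that Health reaches zero or below.
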(event `self.ReceiveBeginPlay`
  ;[1 1 1] On Creation (Spawn Turret)
  (`|SpawnActorFromClass` "/Game/Blueprints/Engineer/Turret.Turret_C" (`KismetMathLibrary.MakeTransform` (`self.K2_GetActorLocation`)) "Undefined" "OverrideRootScale" null null))

(event `self.ReceiveTick`
  (params (DeltaSeconds :type "Float (single-precision)"))
  ;[1 1 1] On Turret Health 0 then destroy this actor
  (bind _asturret (cast `/Game/Blueprints/Engineer/Turret` (`|GetArrayItem` (`self.GetOverlappingActors` "/Game/Blueprints/Engineer/Turret.Turret_C"))))
  (if (<= (`/Game/Blueprints/Engineer/Turret.Health` _asturret) 0.0)
    (`self.K2_DestroyActor`)))

(fn `UserConstructionScript`)