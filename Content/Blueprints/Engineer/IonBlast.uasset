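; Engineer ion blast actor that damages enemies entering its overlap area.
; On BeginPlay it attaches a scaled emitter to its sphere, then uses a looped flag check around a ten-second delay to destroy that emitter.
; Each overlap with a UhouseThirdPersonEnemy subtracts IonDamage directly from its Health.
; Only the emitter is destroyed; the actor itself is never destroyed in these graphs.
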(event `self.ReceiveBeginPlay`
  ;[1 1 1] On Blast Creation
  (set `self.Blast_Exists` true)
  (bind _returnvalue (`GameplayStatics.SpawnEmitterAttached` null (`self.Sphere`) "None" (0.0 0.0 0.0) (struct) (2.0 2.0 2.0)))
  (bind _output_get (set `self.Emitter Ref` _returnvalue))
  (if (`self.Blast_Exists`) :!label _label
    (`KismetSystemLibrary.Delay` 10.0)
    (set `self.Blast_Exists` false)
    (goto _label)
    (else
      (`ActorComponent.K2_DestroyComponent` _output_get))))

(event `self.ReceiveActorBeginOverlap`
  (params (OtherActor :type "Actor Object Reference"))
  ;[1 1 1] On Enemy Overlap
  (bind _asuhouse_third_person_enemy (cast `/Game/Blueprints/UhouseThirdPersonEnemy` OtherActor))
  (set `/Game/Blueprints/UhouseThirdPersonEnemy.Health` (- (`/Game/Blueprints/UhouseThirdPersonEnemy.Health` _asuhouse_third_person_enemy) (`self.IonDamage`)) _asuhouse_third_person_enemy))

(fn `UserConstructionScript`)