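; Engineer turret that reserves player mana and counts toward TurretCount until destroyed, starting at half the player's max health.
; Tick targets the first enemy in its Sphere or spins when idle, using Delay to pace bullets by Level-based fire rate and damage.
; Box overlaps apply enemy projectile damage or a timed Overcharge boosting fire rate and health.
; At zero health it hides, then after Cooldown releases the mana and destroys itself.
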(event `self.ReceiveBeginPlay`
  ;[1 1 1] On Creation
  (bind _asplayer (cast `/Game/Blueprints/Player` (`GameplayStatics.GetPlayerCharacter` 0)))
  (set `/Game/Blueprints/Player.ManaReduction` (+ (`self.Mana Hold`) (`/Game/Blueprints/Player.ManaReduction` _asplayer)) _asplayer)
  (set `self.Health` (/ (`/Game/Blueprints/Player.MaxHealth` _asplayer) 2.0))
  (set `/Game/Blueprints/Player.TurretCount` (+ (`/Game/Blueprints/Player.TurretCount` _asplayer) 1.0) _asplayer))

(event `self.ReceiveTick`
  (params (DeltaSeconds :type "Float (single-precision)"))
  (bind _returnvalue (`self.K2_GetActorLocation`))
  (bind _overlappingactors (`PrimitiveComponent.GetOverlappingActors` (`self.Sphere`) "/Game/Blueprints/UhouseThirdPersonEnemy.UhouseThirdPersonEnemy_C"))
  (bind _returnvalue_2 (`self.K2_GetActorLocation` (`self.Target Enemy`)))
  ;[1 1 1] Turret AI
  (if (> (`self.Health`) 0.0)
    ;;[1 1 1] Put overlapping actors in array and see how many of them are of enemy type.
    (bind _output_get (set `self.Enemy Array` _overlappingactors))
    (if (<= (`KismetArrayLibrary.Array_Length` _overlappingactors) 0)
      (set `self.Enemy Spotted` false)
      (set `self.Target Enemy` null)
      (else
        (bind _asuhouse_third_person_enemy (cast `/Game/Blueprints/UhouseThirdPersonEnemy` (`|GetArrayItem` _output_get)))
        (set `self.Enemy Spotted` true)
        (set `self.Target Enemy` _asuhouse_third_person_enemy)))
    (if (`self.Enemy Spotted`)
      (switch `int` (`KismetMathLibrary.RandomInteger` 0)
        (:`0`
          (`self.K2_SetActorRotation` (`KismetMathLibrary.FindLookAtRotation` _returnvalue _returnvalue_2)))
        (:`1`
          (`self.K2_SetActorRotation` (`KismetMathLibrary.FindLookAtRotation` _returnvalue (+ _returnvalue_2 (0.0 25.0 0.0)))))
        (:`2`
          (`self.K2_SetActorRotation` (`KismetMathLibrary.FindLookAtRotation` _returnvalue (+ _returnvalue_2 (25.0 0.0 0.0))))))
      (if (not (`self.ChargeActive`))
        (switch `int` (`self.Level`)
          (:`1`
            _)
          (:`2`
            (set `self.FireRate` 0.5)
            (set `self.Damage` 7.5))
          (:`3`
            (set `self.FireRate` 0.25)
            (set `self.Damage` 10.0))))
      (`KismetSystemLibrary.Delay` (`self.FireRate`))
      (bind _returnvalue_3 (`|SpawnActorFromClass` "/Game/Blueprints/UhousePlayerBullet.UhousePlayerBullet_C" (`KismetMathLibrary.MakeTransform` (+ _returnvalue (0.0 0.0 25.0)) (`self.K2_GetActorRotation`) (0.2 0.2 0.2)) "Undefined" "OverrideRootScale" null null))
      (set `/Game/Blueprints/UhousePlayerBullet.Damage` (`self.Damage`) _returnvalue_3)
      (else
        (`KismetSystemLibrary.Delay` 0.01)
        (`self.K2_SetActorRotation` (`KismetMathLibrary.MakeRotator` (.roll (`self.K2_GetActorRotation`)) (.pitch (`self.K2_GetActorRotation`)) (+ (.yaw (`self.K2_GetActorRotation`)) 2.0)))))
    (else
      ;[1 1 1] On Destruction
      (`SceneComponent.SetVisibility` (`self.Turret Gun`) false false)
      (`SceneComponent.SetVisibility` (`self.Barrel1`) false false)
      (`SceneComponent.SetVisibility` (`self.Barrel2`) false false)
      (`SceneComponent.SetVisibility` (`self.Effect`) false false)
      (`SceneComponent.SetVisibility` (`self.Barrel3`) false false)
      (`PrimitiveComponent.SetCollisionEnabled` (`self.Effect`) "NoCollision")
      (`PrimitiveComponent.SetCollisionEnabled` (`self.Barrel3`) "NoCollision")
      (`PrimitiveComponent.SetCollisionEnabled` (`self.Barrel2`) "NoCollision")
      (`PrimitiveComponent.SetCollisionEnabled` (`self.Barrel1`) "NoCollision")
      (`PrimitiveComponent.SetCollisionEnabled` (`self.Turret Gun`) "NoCollision")
      (`KismetSystemLibrary.Delay` (`self.Cooldown`))
      (bind _asplayer (cast `/Game/Blueprints/Player` (`GameplayStatics.GetPlayerCharacter` 0)))
      (set `/Game/Blueprints/Player.ManaReduction` (- (`/Game/Blueprints/Player.ManaReduction` _asplayer) (`self.Mana Hold`)) _asplayer)
      (set `/Game/Blueprints/Player.TurretCount` (- (`/Game/Blueprints/Player.TurretCount` _asplayer) 1.0) _asplayer)
      (`self.K2_DestroyActor`))))

(event `self.Box.OnComponentBeginOverlap`
  (params (OverlappedComponent :type "PrimitiveComponent Object Reference") (OtherActor :type "Actor Object Reference") (OtherComp :type "PrimitiveComponent Object Reference") (OtherBodyIndex :type Integer) (bFromSweep :type Boolean) (SweepResult :type "HitResult Structure (by ref)"))
  (bind _temphealth (`self.TempHealth`))
  ;[1 1 1] Enemy Bullet Interaction
  (bind _asuhouse_enemy_projectile_bullet (cast `/Game/Blueprints/UhouseEnemyProjectileBullet` OtherActor)
    (:`then`
      (set `self.Health` (- (`self.Health`) (`/Game/Blueprints/UhouseEnemyProjectileBullet.ProjDamage` _asuhouse_enemy_projectile_bullet)))
      (`self.K2_DestroyActor` _asuhouse_enemy_projectile_bullet))
    (:`CastFailed`
      (bind _asuhouse_enemy_projectile_mage (cast `/Game/Blueprints/UhouseEnemyProjectileMage` OtherActor)
        (:`then`
          (set `self.Health` (- (`self.Health`) (`/Game/Blueprints/UhouseEnemyProjectileMage.ProjDamage` _asuhouse_enemy_projectile_mage)))
          (`self.K2_DestroyActor` _asuhouse_enemy_projectile_mage))
        (:`CastFailed`
          (bind _asovercharge (cast `/Game/Blueprints/Engineer/Overcharge` OtherActor))
          (set `MovementComponent.Velocity` (0.0 0.0 0.0) (`/Game/Blueprints/Engineer/Overcharge.ProjectileMovement` _asovercharge))
          (set `self.ChargeActive` true)
          (set `self.TempRate` (`self.FireRate`))
          (set `self.FireRate` 0.2)
          (set `self.Health` (+ (`self.Health`) _temphealth))
          (`KismetSystemLibrary.Delay` (`/Game/Blueprints/Engineer/Overcharge.ActiveTime` _asovercharge))
          (set `self.Health` (- (`self.Health`) (/ _temphealth 2.0)))
          (set `self.FireRate` (`self.TempRate`))
          (set `self.ChargeActive` false))))))

(fn `UserConstructionScript`)